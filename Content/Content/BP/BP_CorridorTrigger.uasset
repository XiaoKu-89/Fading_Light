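; Corridor trigger volume that switches doors and lighting when the first-person player walks into its box.
; It stays inert until its Arm event is called.
; An armed overlap closes TargetDoor, shows the corridor light in pale blue, unhides SceneBLight, arms every BP_ExitTrigger in the level and forces DoorB open.
; Triggered is set but never checked here, so later overlaps repeat the sequence.
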(event `self.Box.OnComponentBeginOverlap`
  (params (OverlappedComponent :type "PrimitiveComponent Object Reference") (OtherActor :type "Actor Object Reference") (OtherComp :type "PrimitiveComponent Object Reference") (OtherBodyIndex :type Integer) (bFromSweep :type Boolean) (SweepResult :type "HitResult Structure (by ref)"))
  (cast `/Game/FirstPerson/Blueprints/BP_FirstPersonCharacter` OtherActor)
  (if (`self.bArmed`)
    (set `self.bTriggered` true)
    (`/Game/Content/BP/BP_Door.CloseDoor` (`self.TargetDoor`))
    (`SceneComponent.SetVisibility` (`Actor.RootComponent` (`self.CorridorLight`)) true false)
    (`LightComponent.SetLightColor` (`PointLight.PointLightComponent` (`self.CorridorLight`)) (struct :`R` 0.6 :`G` 0.75 :`B` 0.95 :`A` 1.0) true)
    (`self.SetActorHiddenInGame` (`self.SceneBLight`) false)
    (bind _outactors (`GameplayStatics.GetAllActorsOfClass` "/Game/Content/BP/BP_ExitTrigger.BP_ExitTrigger_C"))
    (for _array_element _outactors
      (`/Game/Content/BP/BP_ExitTrigger.Arm` _array_element))
    (bind _output_get (set `self.DoorB` (`self.DoorB`)))
    (`/Game/Content/BP/BP_Door.ForceOpen` _output_get)))

(event `Arm`
  (set `self.bArmed` true))

(fn `UserConstructionScript`)