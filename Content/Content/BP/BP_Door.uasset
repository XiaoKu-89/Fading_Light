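; BP_Door is an interactable door that snaps between closed and open yaw rotations, with a lock and a horror-style light scare.
; Interact plays Sting_Low when locked, otherwise ToggleDoor checks current yaw to call CloseDoor or ForceOpen.
; SlamAndLock shuts and locks it, while ForceOpen unlocks and opens it.
; With a valid RoomLight, the first opening hides that light with a sting; later openings play the sting at world origin.
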(event `ToggleDoor`
  (if (> (.yaw (`self.K2_GetActorRotation`)) 135.0)
    (`self.CloseDoor`)
    (else
      (`self.ForceOpen`))))

(event `SlamAndLock`
  (set `self.bLocked` true)
  (`self.K2_SetActorRelativeRotation` (struct :`Yaw` 90.0))
  (`GameplayStatics.PlaySoundAtLocation` "/Game/Audio/Sting_Low.Sting_Low" (`self.K2_GetActorLocation`) (struct) 1.0 0.5 0.0 null null null null))

(event `ForceOpen`
  (bind _roomlight (`self.RoomLight`))
  (set `self.bLocked` false)
  (`self.K2_SetActorRelativeRotation` (struct :`Yaw` 180.0))
  (`/Engine/EditorBlueprintResources/StandardMacros.IsValid` _roomlight
    (:`Is Valid`
      (if (`self.bLightKilled`)
        (`GameplayStatics.PlaySoundAtLocation` "/Game/Audio/Sting_Low.Sting_Low" (0.0 0.0 0.0) (struct) 1.0 1.0 0.0 null null null null)
        (else
          (set `self.bLightKilled` true)
          (`SceneComponent.SetVisibility` (`PointLight.PointLightComponent` _roomlight) false false)
          (`GameplayStatics.PlaySoundAtLocation` "/Game/Audio/Sting_Low.Sting_Low" (`self.K2_GetActorLocation`) (struct) 1.0 0.5 0.0 null null null null))))))

(event `CloseDoor`
  (`self.K2_SetActorRelativeRotation` (struct :`Yaw` 90.0))
  (`GameplayStatics.PlaySoundAtLocation` "/Game/Audio/Sting_Low.Sting_Low" (`self.K2_GetActorLocation`) (struct) 1.0 1.0 0.0 null null null null))

(event `/Game/Content/BPI/BPI_Interactable.Interact`
  (if (`self.bLocked`)
    (`GameplayStatics.PlaySoundAtLocation` "/Game/Audio/Sting_Low.Sting_Low" (`self.K2_GetActorLocation`) (struct) 0.35 1.8 0.0 null null null null)
    (else
      (`self.ToggleDoor`))))

(fn `UserConstructionScript`)