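; BP_ExitPickup is an interactable exit pickup that triggers the final scare when used.
; Overlap with its Sphere component shows the Re component, and leaving hides it again, with no filter on the overlapping actor.
; Interact adds a WBP_HuiTo widget to the first player's viewport, then calls FinalScare on all BP_FinalRoomTrigger actors found through GetAllActorsOfClass.
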(event `self.Sphere.OnComponentBeginOverlap`
  (params (OverlappedComponent :type "PrimitiveComponent Object Reference") (OtherActor :type "Actor Object Reference") (OtherComp :type "PrimitiveComponent Object Reference") (OtherBodyIndex :type Integer) (bFromSweep :type Boolean) (SweepResult :type "HitResult Structure (by ref)"))
  (`SceneComponent.SetVisibility` (`self.re`) true false))

(event `self.Sphere.OnComponentEndOverlap`
  (params (OverlappedComponent :type "PrimitiveComponent Object Reference") (OtherActor :type "Actor Object Reference") (OtherComp :type "PrimitiveComponent Object Reference") (OtherBodyIndex :type Integer))
  (`SceneComponent.SetVisibility` (`self.re`) false false))

(event `self.Interact`
  (bind _returnvalue (`|CreateWidget` "/Game/UI/WBP_HuiTo.WBP_HuiTo_C" (`GameplayStatics.GetPlayerController` 0)))
  (`UserWidget.AddToViewport` _returnvalue 0)
  (bind _outactors (`GameplayStatics.GetAllActorsOfClass` "/Game/Content/BP/BP_FinalRoomTrigger.BP_FinalRoomTrigger_C"))
  (`/Game/Content/BP/BP_FinalRoomTrigger.FinalScare` _outactors))

(fn `UserConstructionScript`)