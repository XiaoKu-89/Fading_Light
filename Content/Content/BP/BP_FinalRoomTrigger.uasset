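; Trigger actor that stages the final room scare and ends the game.
; Its box overlap fires once, stopping the player's light watch, slamming and locking FinalDoor, hiding Figure and switching from RedLight to ExitLight.
; FinalScare, not called within this Blueprint, waits, locks look input and turns the player toward the revealed, red-lit Figure with a sting.
; Timed delays then show the exit and end widgets before quitting.
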(event `self.Box.OnComponentBeginOverlap`
  (params (OverlappedComponent :type "PrimitiveComponent Object Reference") (OtherActor :type "Actor Object Reference") (OtherComp :type "PrimitiveComponent Object Reference") (OtherBodyIndex :type Integer) (bFromSweep :type Boolean) (SweepResult :type "HitResult Structure (by ref)"))
  (bind _figure (`self.Figure`))
  (if (not (`self.bTriggered`))
    (set `self.bTriggered` true)
    (bind _asbp_first_person_character (cast `/Game/FirstPerson/Blueprints/BP_FirstPersonCharacter` OtherActor))
    (`/Game/FirstPerson/Blueprints/BP_FirstPersonCharacter.StopLightWatch` _asbp_first_person_character)
    (`/Game/Content/BP/BP_Door.SlamAndLock` (`self.FinalDoor`))
    (`self.SetActorHiddenInGame` _figure true)
    (`self.SetActorEnableCollision` _figure false)
    (`SceneComponent.SetVisibility` (`Actor.RootComponent` (`self.RedLight`)) false false)
    (`SceneComponent.SetVisibility` (`Actor.RootComponent` (`self.ExitLight`)) true false)))

(event `FinalScare`
  (bind _figure (`self.Figure`))
  (`KismetSystemLibrary.Delay` 2.9)
  (`Controller.SetIgnoreLookInput` (`GameplayStatics.GetPlayerController` 0) true)
  (`Controller.SetControlRotation` (`GameplayStatics.GetPlayerController` 0) (`KismetMathLibrary.MakeRotator` 0.0 0.0 (.yaw (`KismetMathLibrary.FindLookAtRotation` (`self.K2_GetActorLocation` (`GameplayStatics.GetPlayerPawn` 0)) (`self.K2_GetActorLocation` (`self.Figure`))))))
  (`self.SetActorHiddenInGame` _figure false)
  (`self.K2_SetActorRelativeRotation` _figure (struct :`Yaw` 180.0) false false)
  (`self.SetActorEnableCollision` (`self.Figure`) false)
  (`SceneComponent.SetVisibility` (`SpotLight.SpotLightComponent` (`self.RedLight`)) true false)
  (`GameplayStatics.PlaySoundAtLocation` "/Game/Audio/Sting_Low.Sting_Low" (`self.K2_GetActorLocation`) (struct) 1.0 1.0 0.0 null null null null)
  (`KismetSystemLibrary.Delay` 4.5)
  (bind _returnvalue (`|CreateWidget` "/Game/UI/WBP_Exit.WBP_Exit_C" (`GameplayStatics.GetPlayerController` 0)))
  (`UserWidget.AddToPlayerScreen` _returnvalue 0)
  (`KismetSystemLibrary.Delay` 2.0)
  (bind _returnvalue_2 (`|CreateWidget` "/Game/UI/WBP_End.WBP_End_C" (`GameplayStatics.GetPlayerController` 0)))
  (`UserWidget.AddToPlayerScreen` _returnvalue_2 0)
  (`KismetSystemLibrary.Delay` 2.0)
  (`KismetSystemLibrary.QuitGame` null "Quit"))

(fn `UserConstructionScript`)