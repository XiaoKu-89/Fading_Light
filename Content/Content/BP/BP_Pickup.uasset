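; BP_Pickup is an interactable pickup that opens a note panel and triggers level progression.
; Its sphere overlap shows and hides the Re component, without filtering by actor.
; Interact adds a WBP_NotePanel widget to the viewport, force-opens TargetDoor and arms every BP_CorridorTrigger in the level.
; DestroyActor is called inside that loop body, so the pickup only destroys itself if at least one trigger exists.
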(event `self.Sphere.OnComponentBeginOverlap`
  (params (OverlappedComponent :type "PrimitiveComponent Object Reference") (OtherActor :type "Actor Object Reference") (OtherComp :type "PrimitiveComponent Object Reference") (OtherBodyIndex :type Integer) (bFromSweep :type Boolean) (SweepResult :type "HitResult Structure (by ref)"))
  (`SceneComponent.SetVisibility` (`self.re`) true false))

(event `self.Sphere.OnComponentEndOverlap`
  (params (OverlappedComponent :type "PrimitiveComponent Object Reference") (OtherActor :type "Actor Object Reference") (OtherComp :type "PrimitiveComponent Object Reference") (OtherBodyIndex :type Integer))
  (`SceneComponent.SetVisibility` (`self.re`) false false))

(event `/Game/Content/BPI/BPI_Interactable.Interact`
  (bind _returnvalue (`|CreateWidget` "/Game/UI/WBP_NotePanel.WBP_NotePanel_C" (`GameplayStatics.GetPlayerController` 0)))
  (`UserWidget.AddToViewport` _returnvalue 0)
  (`/Game/Content/BP/BP_Door.ForceOpen` (`self.TargetDoor`))
  (bind _outactors (`GameplayStatics.GetAllActorsOfClass` "/Game/Content/BP/BP_CorridorTrigger.BP_CorridorTrigger_C"))
  (for _array_element _outactors
    (`/Game/Content/BP/BP_CorridorTrigger.Arm` _array_element)
    (`self.K2_DestroyActor`)))

(fn `UserConstructionScript`)